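; Whip actor with a cable rope and kunai that shoots toward targets the player's camera points at.
; UseWhip sphere-traces from the camera and, if the hit actor implements BPI_Whip, stores the hit location and distance and plays WhipTimeline.
; Each update, MoveRope shows the rope, scales its length by a curve and lerps the kunai toward the hit by another.
; ResetRope plays the timeline in reverse.
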(event Custom|UseWhip
  (bind _returnvalue (Game|GetPlayerCharacter 0))
  (bind _returnvalue_2 (Actor|GetComponentbyClass _returnvalue "/Script/Engine.CameraComponent"))
  (bind _returnvalue_3 (Transformation|GetWorldLocation _returnvalue_2))
  (bind _outhit (Collision|SphereTraceByChannel _returnvalue_3 (+ _returnvalue_3 (* (Math|Vector|GetForwardVector _returnvalue_2) 1e+05)) 5e+01 "TraceTypeQuery1" false 0 "ForDuration"))
  (if (Utilities|DoesObjectImplementInterface (.HitActor (Collision|BreakHitResult _outhit)) "/Game/Sekiro/Blueprints/BPI_Whip.BPI_Whip_C")
    (Variables|Default|Set_hitLocation (.Location (Collision|BreakHitResult _outhit)))
    (Variables|Default|Set_distanceFromHitLocation (Math|Vector|VectorLength (- (Transformation|GetActorLocation) (.Location (Collision|BreakHitResult _outhit)))))
    (bind _alpha (Timeline|WhipTimeline PlayFromStart)
      (:Update
        (CallFunction|MoveRope _alpha))
      (:Finished
        (Utilities|FlowControl|Delay 0.2)))))

(event Custom|ResetRope
  (bind _alpha (Timeline|WhipTimeline ReverseFromEnd)
    (:Update
      (CallFunction|MoveRope _alpha))
    (:Finished
      (Utilities|FlowControl|Delay 0.2))))

(fn ConstructionScript)

(fn MoveRope
  (params (InTime :type Float%20%28single-precision%29))
  (bind _kunai (Variables|Default|GetKunai))
  (LocalVariables|Set_alpha InTime)
  (Rendering|SetVisibility (Variables|Default|GetRope) true false)
  (Variables|/Script/CableComponent.CableComponent|SetCableLength (Variables|Default|GetRope) (* (Math|Curves|GetFloatValue (Variables|Default|GetAirRopeLength) (LocalVariables|Get_alpha)) (Variables|Default|Get_distanceFromHitLocation)))
  (Transformation|SetWorldLocation _kunai (Math|Vector|Lerp(Vector) (Transformation|GetWorldLocation _kunai) (Variables|Default|Get_hitLocation) (Math|Curves|GetFloatValue (Variables|Default|GetAirRopePosition) (LocalVariables|Get_alpha))) false false))